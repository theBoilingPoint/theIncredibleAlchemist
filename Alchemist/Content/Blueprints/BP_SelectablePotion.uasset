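; BP_SelectablePotion is a potion the player picks up and pours into a cauldron, with ElementIdx choosing red, blue or yellow.
; The construction script sets the sphere material from that index, and selection attaches it to the first-person character's arm with physics off.
; Deselection line-traces from the camera: a cauldron triggers a tilt timeline, then destruction and an AddColor broadcast.
; Other valid hits drop it with physics; misses leave it held.
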(event EventBeginPlay
  (|CallParentFunction) ; This node is disabled and will not be called.\nDrag off pins to build functionality.
)

(event Collision|EventActorBeginOverlap
  (params (OtherActor :type Actor%20Object%20Reference))
  (|CallParentFunction OtherActor) ; This node is disabled and will not be called.\nDrag off pins to build functionality.
)

(event EventTick
  (params (DeltaSeconds :type Float%20%28single-precision%29))
  (|CallParentFunction DeltaSeconds) ; This node is disabled and will not be called.\nDrag off pins to build functionality.
)

(event EventSelectMyActor
  (bind _asbp_first_person_character (Utilities|Casting|CastToBP_FirstPersonCharacter (Game|Player|GetPlayerPawn 0)))
  (Transformation|AttachComponentToComponent (Variables|/Game/FirstPerson/Blueprints/BP_FirstPersonCharacter.BP_FirstPersonCharacter_C|Getarm _asbp_first_person_character) "None" "SnapToTarget" "SnapToTarget" "KeepRelative" true)
  (Physics|SetSimulatePhysics (Variables|Default|GetSphere) false))

(event EventDeselectMyActor
  (bind _returnvalue (Game|GetPlayerCameraManager 0))
  (bind _elementidx (Variables|Default|GetElementIdx))
  (bind _returnvalue_2 (Camera|GetCameraLocation _returnvalue))
  (bind _outhit (Collision|LineTraceForObjects _returnvalue_2 (+ _returnvalue_2 (* (Math|Vector|GetForwardVector (Variables|/Script/Engine.PlayerCameraManager|GetTransformComponent _returnvalue)) "2500.000000,2500.000000,2500.000000")) (Utilities|Array|MakeArray "ObjectTypeQuery2") false 0 "None"))
  (Utilities|IsValid (.hitactor _outhit)
    (:Is%20Valid
      (Development|PrintString "Hit")
      (Utilities|Casting|CastToBP_Cauldron (.hitactor _outhit)
        (:then
          (bind _pouralpha (Timeline|PourTimeline Play)
            (:Update
              (Transformation|SetActorRotation (Math|Rotator|Lerp(Rotator) (Transformation|GetActorRotation) "-90.000000,0.000000,-90.000000" _pouralpha)))
            (:Finished
              (Actor|DestroyActor)
              (if (== _elementidx 0)
                (Default|CallOnAddColor (Math|Vector|MakeVector 1.0 0.02 0.001))
                (Development|PrintString "red added")
                (elif (== _elementidx 1)
                  (Default|CallOnAddColor (Math|Vector|MakeVector 0.051 0.106 0.267))
                  (Development|PrintString "blue added")
                  (elif (== _elementidx 2)
                    (Default|CallOnAddColor (Math|Vector|MakeVector 0.996 0.925 0.0))
                    (Development|PrintString "yellow added")))))))
        (:CastFailed
          (Transformation|DetachFromActor "KeepRelative" "KeepRelative" "KeepRelative")
          (Physics|SetSimulatePhysics (Variables|Default|GetSphere) true))))
    (:Is%20Not%20Valid
      (Development|PrintString "Not Valid"))))

(event Input|KeyboardEvents|3
  (params (Key :type Key%20Structure :default "None"))
  (:Pressed
    (Development|PrintString "calling dispatcher")
    (Default|CallOnAddColor)))

(fn ConstructionScript
  (bind _elementidx (Variables|Default|GetElementIdx))
  (bind _sphere (Variables|Default|GetSphere))
  (Development|PrintString (Utilities|String|ToString(Integer) _elementidx))
  (if (== _elementidx 0)
    (Rendering|Material|SetMaterial _sphere 0 "/Game/LevelPrototyping/Materials/M_FlatColRed.M_FlatColRed")
    (Development|PrintString "Set to Red")
    (elif (== _elementidx 1)
      (Rendering|Material|SetMaterial _sphere 0 "/Game/LevelPrototyping/Materials/M_FlatColBlue.M_FlatColBlue")
      (Development|PrintString "Set to Blue")
      (elif (== _elementidx 2)
        (Rendering|Material|SetMaterial _sphere 0 "/Game/LevelPrototyping/Materials/M_FlatColYellow.M_FlatColYellow")
        (Development|PrintString "Set to Yellow")))))

(fn IsSelected?
  (return false))